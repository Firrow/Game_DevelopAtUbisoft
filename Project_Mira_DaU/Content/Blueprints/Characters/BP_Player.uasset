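; Player Blueprint for a 2D flipbook character, handling the sprite animation for idle, walking, jump rise, falling and ladder states.
; Every Tick it rotates the sprite to match IsFacingLeft and swaps the flipbook only when CurrentStateMovement differs from the cached OldAnimation.
; The onPause state stops playback instead of changing the flipbook.
; Movement state and facing are only read here, not set.
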(event `self.ReceiveBeginPlay`)

(event `self.ReceiveTick`
  (params (DeltaSeconds :type "Float (single-precision)"))
  (bind _currentstatemovement (`self.CurrentStateMovement`))
  (bind _sprite (`self.Sprite`))
  (`self.RotateAnimation`)
  (if (`KismetStringLibrary.NotEqual_StrStr` (`self.CurrentStateMovement`) "onPause")
    (`PaperFlipbookComponent.Play` _sprite)
    (if (`KismetStringLibrary.NotEqual_StrStr` (`self.CurrentStateMovement`) (`self.OldAnimation`))
      (set `self.OldAnimation` _currentstatemovement)
      (`self.UpdateAnimation` _currentstatemovement))
    (else
      (`PaperFlipbookComponent.Stop` _sprite))))

(fn `RotateAnimation`
  (if (`self.isFacingLeft`)
    (`SceneComponent.K2_SetRelativeRotation` (`self.Sprite`) (struct :`Yaw` 180.0) false false)
    (else
      (`SceneComponent.K2_SetRelativeRotation` :`self` (`self.Sprite`)))))

(fn `UpdateAnimation`
  (params (Selection :type String))
  (bind _sprite (`self.Sprite`))
  (switch `string` Selection
    (:`idle`
      (`PaperFlipbookComponent.SetFlipbook` _sprite "/Game/PLACEHOLDERS/Animations/FB_Idle.FB_Idle"))
    (:`move`
      (`PaperFlipbookComponent.SetFlipbook` _sprite "/Game/PLACEHOLDERS/Animations/FB_Walk.FB_Walk"))
    (:`jumpRise`
      (`PaperFlipbookComponent.SetFlipbook` _sprite "/Game/PLACEHOLDERS/Animations/FB_JumpRise.FB_JumpRise"))
    (:`fall`
      (`PaperFlipbookComponent.SetFlipbook` _sprite "/Game/PLACEHOLDERS/Animations/FB_Fall.FB_Fall"))
    (:`ladder`
      (`PaperFlipbookComponent.SetFlipbook` _sprite "/Game/PLACEHOLDERS/Animations/FB_Ladder.FB_Ladder"))))

(fn `UserConstructionScript`)